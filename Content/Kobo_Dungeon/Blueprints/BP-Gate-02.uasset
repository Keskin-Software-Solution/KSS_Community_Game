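; BP-Gate-02 is a dungeon gate Blueprint whose swing is set by a DoorOpenAngle value.
; The construction script yaws GatePivot to the negated angle, clamped between closed and a maximum opening, so edits preview in the editor.
; Tick reapplies the same rotation every frame, so runtime changes to the angle move the gate immediately, with no interpolation or built-in trigger logic.
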(event `self.ReceiveBeginPlay`)

(event `self.ReceiveTick`
  (params (DeltaSeconds :type "Float (single-precision)"))
  (`SceneComponent.K2_SetRelativeRotation` (`self.GatePivot`) (`KismetMathLibrary.MakeRotator` 0.0 0.0 (* (`KismetMathLibrary.FClamp` (`self.Door Open Angle`) 0.0 120.0) -1.0)) false false))

(fn `UserConstructionScript`
  (`SceneComponent.K2_SetRelativeRotation` (`self.GatePivot`) (`KismetMathLibrary.MakeRotator` 0.0 0.0 (* (`KismetMathLibrary.FClamp` (`self.Door Open Angle`) 0.0 120.0) -1.0)) false false))