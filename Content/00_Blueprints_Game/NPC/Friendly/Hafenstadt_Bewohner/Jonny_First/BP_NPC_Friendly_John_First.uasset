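; Blueprint for John First, a friendly NPC filed under the harbor town residents (Hafenstadt_Bewohner).
; On BeginPlay it runs the parent logic, then copies health and max health from its NPC data asset and sets normalized health to full.
; It also applies the skeletal mesh from that data asset.
; Overlap and Tick events are disabled, and the construction script only calls the parent.
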(event `self.ReceiveBeginPlay`
  (bind _npc_data_asset_ref (`self.NPC Data Asset REF`))
  (`parent.ReceiveBeginPlay`)
  (set `self.NPC Health` (`/Game/00_Blueprints_Game/NPC/RescourceNPCDataAsset.NPC Health` _npc_data_asset_ref))
  (set `self.NPC Max Health` (`/Game/00_Blueprints_Game/NPC/RescourceNPCDataAsset.NPC Max Health` _npc_data_asset_ref))
  (set `self.NPC Health Normalized` 1.0)
  (`SkeletalMeshComponent.SetSkeletalMeshAsset` (`self.Mesh`) (`/Game/00_Blueprints_Game/NPC/RescourceNPCDataAsset.NPC Skeletal Mesh` _npc_data_asset_ref)))

(fn `UserConstructionScript`
  (`parent.UserConstructionScript`))