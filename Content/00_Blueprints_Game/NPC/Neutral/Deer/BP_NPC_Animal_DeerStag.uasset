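; Deer stag variant of the neutral animal NPC Blueprint.
; Its construction script runs the parent script, assigns the DeerStag NPC data asset, and if that asset is valid applies its data to the character mesh through SetNPCDataFromDataAsset.
; The event graph holds only disabled placeholder events, so all behaviour comes from the parent class and the data asset.
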(fn `UserConstructionScript`
  (locals (`NPC Data Asset Local` :type "/Game/00_Blueprints_Game/NPC/RescourceNPCDataAsset Object Reference"))
  (`parent.UserConstructionScript`)
  (bind _output_get (set `self.NPC DataAsset` "/Game/00_Blueprints_Game/NPC/Neutral/Deer/NPC_DataAsset_Neutral_DeerStag.NPC_DataAsset_Neutral_DeerStag"))
  (set `local.NPC Data Asset Local` _output_get)
  (bind _npc_data_asset_local (`local.NPC Data Asset Local`)
    (:`then`
      (`self.Set NPC Data From Data Asset` (`self.Mesh`) _npc_data_asset_local))
    (:`else`)))