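; Template NPC actor that can be targeted, takes damage and grants the player XP on death.
; A data asset supplies name, level and energy at construction, with a separate function also setting mesh and health.
; Tick refreshes the world-space nameplate and turns it to the camera; clicking sets the controller's target and shows an indicator.
; Damage checks health before subtracting, and death destroys the actor immediately after starting its montage.
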(event `NPC Dead`
  ;[1 1 1] Event NPC died
  (`/Game/ThirdPerson/Blueprints/BP_ThirdPersonCharacter.Increase Player XP` (`self.As BP Third Person Character`) (`self.Increasing XP - Implement in Structure`))
  (`self.PlayAnimMontage` (`self. Death Anim Montage`))
  (`self.K2_DestroyActor`))

(event `self.ReceiveAnyDamage`
  (params (Damage :type "Float (single-precision)") (DamageType :type "DamageType Object Reference") (InstigatedBy :type "Controller Object Reference") (DamageCauser :type "Actor Object Reference"))
  ;[1 1 1] Schaden erleiden
  (if (<= (`self.NPC Health`) 0.0)
    (`self.NPC Dead`)
    (else
      (bind _output_get (set `self.NPC Health` (- (`self.NPC Health`) Damage)))
      (set `self.NPC Health Normalized` (`KismetMathLibrary.NormalizeToRange` _output_get 0.0 (`self.NPC Max Health`)))
      (`self.TargetDamaged`))))

(event `RotateHealthToPlayer`
  (bind _healthbar___ui_widget (`self.Healthbar & UI Widget`))
  ;[1 1 1] Dieser Block richtet die Healthbar in in Blickrichtung Spieler
  (`SceneComponent.K2_SetWorldRotation` _healthbar___ui_widget (`KismetMathLibrary.FindLookAtRotation` (`SceneComponent.K2_GetComponentLocation` _healthbar___ui_widget) (`SceneComponent.K2_GetComponentLocation` (`PlayerCameraManager.TransformComponent` (`GameplayStatics.GetPlayerCameraManager` 0)))) false false))

(event `setUp NPC Healthbar`
  (bind _as_wbp_npc_health_bar (`self.As WBP NPC Health Bar`))
  ;[1 1 1] Dieser Block updatet die Healthbar bei jedem Tick
  (`ProgressBar.SetPercent` (`/Game/00_Blueprints_Game/UI/HealthbarsUI/WBP_NPC_Nameplate_HealthBar.NPCHealthbar` _as_wbp_npc_health_bar) (/ (`self.NPC Health`) (`self.NPC Max Health`)))
  (set `TextBlock.Text` (`KismetTextLibrary.Conv_StringToText` (`self.NPC Name`)) (`/Game/00_Blueprints_Game/UI/HealthbarsUI/WBP_NPC_Nameplate_HealthBar.TargetNameWorldUI` _as_wbp_npc_health_bar))
  (`self.RotateHealthToPlayer`)
  (set `TextBlock.Text` (`KismetTextLibrary.Conv_IntToText` (`self.NPC Level`)) (`/Game/00_Blueprints_Game/UI/HealthbarsUI/WBP_NPC_Nameplate_HealthBar.NPCLevelUI` (`self.As WBP NPC Health Bar`))))

(event `self.ReceiveBeginPlay`
  ;[1 1 1] Events
  (bind _aswbp_npc_nameplate_health_bar (cast `/Game/00_Blueprints_Game/UI/HealthbarsUI/WBP_NPC_Nameplate_HealthBar` (`WidgetComponent.GetWidget` (`self.Healthbar & UI Widget`))))
  (set `self.As WBP NPC Health Bar` _aswbp_npc_nameplate_health_bar)
  (bind _asbp_third_person_character (cast `/Game/ThirdPerson/Blueprints/BP_ThirdPersonCharacter` (`GameplayStatics.GetPlayerCharacter` 0)))
  (set `self.As BP Third Person Character` _asbp_third_person_character))

(event `self.ReceiveTick`
  (params (DeltaSeconds :type "Float (single-precision)"))
  ;[1 1 1] Events
  (`self.setUp NPC Healthbar`))

(event `self.ReceiveActorOnClicked`
  (params (ButtonPressed :type "Key Structure"))
  ;[1 1 1] On Click Event Markiere Target und setzte es in Player Kampf Target
  (bind _asmy_controller (cast `/Game/ThirdPerson/Blueprints/MyController` (`GameplayStatics.GetPlayerController` 0)))
  (`/Game/ThirdPerson/Blueprints/MyController.SetTarget` _asmy_controller self)
  (add `/Game/ThirdPerson/Blueprints/MyController.TargetChanged` _asmy_controller (delegate `ClearTarget`))
  (`SceneComponent.SetVisibility` (`self.Target Indicator`) true false))

(event `ClearTarget`
  ;[1 1 1] On Click Event Markiere Target und setzte es in Player Kampf Target
  (`SceneComponent.SetVisibility` (`self.Target Indicator`) false false))

(fn `Set NPC Data From Data Asset`
  (params (`Target Skeletal Mesh` :type "SkeletalMeshComponent Object Reference") (`NPC Data Asset REF` :type "/Game/00_Blueprints_Game/NPC/RescourceNPCDataAsset Object Reference"))
  (bind _npc_dataasset (`self.NPC DataAsset`))
  ;[1 1 1] Comment
  (bind _output_get (set `self.NPC Data Asset REF` `NPC Data Asset REF`))
  (`SkeletalMeshComponent.SetSkeletalMeshAsset` `Target Skeletal Mesh` (`/Game/00_Blueprints_Game/NPC/RescourceNPCDataAsset.NPC Skeletal Mesh` _output_get))
  (set `self.NPC Name` (`KismetTextLibrary.Conv_TextToString` (`/Game/00_Blueprints_Game/NPC/RescourceNPCDataAsset.NPC Name` _npc_dataasset)))
  (set `self.NPC Health` (`/Game/00_Blueprints_Game/NPC/RescourceNPCDataAsset.NPC Health` _npc_dataasset))
  (set `self.NPC Max Health` (`/Game/00_Blueprints_Game/NPC/RescourceNPCDataAsset.NPC Max Health` _npc_dataasset))
  (set `self.NPC Level` (`/Game/00_Blueprints_Game/NPC/RescourceNPCDataAsset.NPC Level` _npc_dataasset))
  (set `/Game/00_Blueprints_Game/NPC/RescourceNPCDataAsset.NPC Disposition` (`/Game/00_Blueprints_Game/NPC/RescourceNPCDataAsset.NPC Disposition` _npc_dataasset) _npc_dataasset))

(fn `UserConstructionScript`
  (bind _npc_dataasset (`self.NPC DataAsset`))
  (bind _npc_dataasset_2 (`self.NPC DataAsset`))
  (set `self.NPC Name` (`KismetTextLibrary.Conv_TextToString` (`/Game/00_Blueprints_Game/NPC/RescourceNPCDataAsset.NPC Name` _npc_dataasset_2)))
  (set `self.NPC Level` (`/Game/00_Blueprints_Game/NPC/RescourceNPCDataAsset.NPC Level` _npc_dataasset_2))
  (set `self.NPC Mana/Energie` (`/Game/00_Blueprints_Game/NPC/RescourceNPCDataAsset.NPC Energie` _npc_dataasset))
  (set `self.NPC Max Mana/Energie` (`/Game/00_Blueprints_Game/NPC/RescourceNPCDataAsset.NPC Max Energie` _npc_dataasset)))