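; Enemy NPC template Blueprint that chases and melee-attacks the player once Pawn Sensing spots a pawn.
; Each sighting sets a seen flag and starts an AI MoveTo toward the player; successful arrival triggers a goblin slash montage with immediate fixed damage.
; Tick halts movement until the first sighting, as the flag is never cleared here.
; The look-at rotation logic is disconnected and never runs.
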(event `self.ReceiveTick`
  (params (DeltaSeconds :type "Float (single-precision)"))
  (`parent.ReceiveTick` DeltaSeconds)
  (if (not (`self.isSeeingPlayer`))
    (`MovementComponent.StopMovementImmediately` (`self.CharacterMovement`))))

(event `self.PawnSensing.OnSeePawn`
  (params (Pawn :type "Pawn Object Reference"))
  ;[1 1 1] Dieser Block ist für die verfolgung des Spielers zuständig
  (set `self.isSeeingPlayer` true)
  (`self.NPCEnemyFollowPlayer`))

(event `NPCEnemyFollowPlayer`
  ;[1 1 1] Dieser Block ist für die verfolgung des Spielers zuständig
  (set `self.canAttack?` true)
  (if (`self.isSeeingPlayer`)
    (`|AIMoveTo` self (0.0 0.0 0.0) (`GameplayStatics.GetPlayerCharacter` 0) 125.0
      (:`OnSuccess`
        (if (`self.canAttack?`)
          (set `self.canAttack?` false)
          (`self.NPC attack Player`))))
    (else
      (set `self.isSeeingPlayer` true))))

(event `NPC attack Player`
  ;[1 1 1] NPC greift Player an
  (bind _returnvalue (`self.PlayAnimMontage` "/Game/00_Blueprints_Game/NPC/Enemy/Goblin/Animations/AnimMontage/AnimMontage_Goblin_body_attack_slash.AnimMontage_Goblin_body_attack_slash"))
  (set `self.AnimPlayTime` _returnvalue)
  (`GameplayStatics.ApplyDamage` (`self.As BP Third Person Character`) 10.0)
  (`KismetSystemLibrary.Delay` (`self.AnimPlayTime`))
  (set `self.canAttack?` false))

(fn `UserConstructionScript`
  (`parent.UserConstructionScript`))